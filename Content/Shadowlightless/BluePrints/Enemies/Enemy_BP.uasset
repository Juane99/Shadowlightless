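; Side-scrolling Paper2D enemy that chases the player along X, attacks in melee and awards points to an overlapping player when destroyed.
; Tick drives death, following, attacking and flipbook/facing updates from flags set by the detection and attack collision overlaps.
; A looping delay damages the player while in attack range.
; At zero health it drops collision responses, plays death flipbooks, spawns explosion emitters and destroys itself after a delay.
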(event `self.ReceiveBeginPlay`
  ;[1 1 1] Begin Play
  (`ActorComponent.SetIsReplicated` (`self.Sprite`) true))

(event `UpdateAnimation`
  (params (Jump :type "PaperFlipbook Object Reference") (Idle :type "PaperFlipbook Object Reference") (Run :type "PaperFlipbook Object Reference"))
  ;[1 1 1] Handle Animation
  ;;[1 1 1] Jump, Run, Idle, Slide
  (`PaperFlipbookComponent.SetFlipbook` (`self.Sprite`) (select `bool` (`NavMovementComponent.IsFalling` (`self.CharacterMovement`)) :`false` (select `bool` (> (`KismetMathLibrary.VSize` (`self.GetVelocity`)) 0.0) :`false` Idle :`true` Run) :`true` Jump)))

(event `self.ReceiveTick`
  (params (DeltaSeconds :type "Float (single-precision)"))
  (bind _capsulecomponent (`self.CapsuleComponent`))
  ;[1 1 1] Event Tick
  ;;[1 1 1] Death
  (if (<= (`self.Health`) 0.0)
    (set `self.bisDead` true))
  (if (`self.bisDead`)
    (set `self.isOverlappingAttack` false)
    (`PrimitiveComponent.SetCollisionResponseToChannel` _capsulecomponent "ECC_Pawn" "ECR_Ignore")
    (`PrimitiveComponent.SetCollisionResponseToChannel` _capsulecomponent "ECC_PhysicsBody" "ECR_Ignore")
    (`PrimitiveComponent.SetCollisionResponseToChannel` _capsulecomponent "ECC_WorldDynamic" "ECR_Ignore")
    (`self.DeathAnimation` null)
    (`GameplayStatics.SpawnEmitterAtLocation` "/Game/StarterContent/Particles/P_Explosion.P_Explosion" (`self.K2_GetActorLocation`))
    ;;;[1 1 1] Character destroy
    (`KismetSystemLibrary.Delay` 3.0)
    (`self.K2_DestroyActor`)
    (else
      (if (`self.isOverlapping`)
        ;;[1 1 1] Follow Character
        (`self.FollowCharacter` null))
      (if (`self.bisattacking`)
        ;;[1 1 1] Attack Character
        (`self.AttackEvent` null)
        (else
          ;;[1 1 1] Update Animation and Rotate
          (`self.UpdateAnimation` null)
          (`self.RotateEvent`))))))

(event `self.ReceiveDestroyed`
  ;[1 1 1] Enemy destroyed
  (bind _ascharacter_bp (cast `/Game/Shadowlightless/BluePrints/Characters/Character_BP` (`|GetArrayItem` (`self.GetOverlappingActors` "/Game/Shadowlightless/BluePrints/Characters/Character_BP.Character_BP_C"))))
  (set `/Game/Shadowlightless/BluePrints/Characters/Character_BP.Points` (+ (`/Game/Shadowlightless/BluePrints/Characters/Character_BP.Points` _ascharacter_bp) 5) _ascharacter_bp))

(event `AttackEvent`
  (params (AttackMelee :type "PaperFlipbook Object Reference") (AttackJumpMelee :type "PaperFlipbook Object Reference"))
  (bind _sprite (`self.Sprite`))
  ;[1 1 1] Handle Animation
  ;;[1 1 1] Attack
  (if (`NavMovementComponent.IsFalling` (`self.CharacterMovement`))
    (`PaperFlipbookComponent.SetFlipbook` _sprite AttackJumpMelee)
    (else
      (`PaperFlipbookComponent.SetFlipbook` _sprite AttackMelee)
      (`MovementComponent.StopMovementImmediately` (`self.CharacterMovement`)))))

(event `self.Box_Collision.OnComponentBeginOverlap`
  (params (OverlappedComponent :type "PrimitiveComponent Object Reference") (OtherActor :type "Actor Object Reference") (OtherComp :type "PrimitiveComponent Object Reference") (OtherBodyIndex :type Integer) (bFromSweep :type Boolean) (SweepResult :type "HitResult Structure (by ref)"))
  ;[1 1 1] Collisions Overlapping
  (if (`ActorComponent.ComponentHasTag` OtherComp "Hitbox")
    (set `self.isOverlapping` true)))

(event `self.Box_Collision.OnComponentEndOverlap`
  (params (OverlappedComponent :type "PrimitiveComponent Object Reference") (OtherActor :type "Actor Object Reference") (OtherComp :type "PrimitiveComponent Object Reference") (OtherBodyIndex :type Integer))
  ;[1 1 1] Collisions Overlapping
  (if (`ActorComponent.ComponentHasTag` OtherComp "Hitbox")
    (set `self.isOverlapping` false)))

(event `self.Attack_Collision.OnComponentBeginOverlap`
  (params (OverlappedComponent :type "PrimitiveComponent Object Reference") (OtherActor :type "Actor Object Reference") (OtherComp :type "PrimitiveComponent Object Reference") (OtherBodyIndex :type Integer) (bFromSweep :type Boolean) (SweepResult :type "HitResult Structure (by ref)"))
  ;[1 1 1] Collisions Overlapping
  (if (`ActorComponent.ComponentHasTag` OtherComp "Hitbox")
    (set `self.isOverlappingAttack` true)
    (`/Engine/EditorBlueprintResources/StandardMacros.DoOnce` false :!label _label
      (:`Completed`
        (set `self.bisattacking` true)
        (`KismetSystemLibrary.Delay` 0.5 :!label _label_2)
        (if (`self.isOverlappingAttack`)
          (bind _ascharacter_bp (cast `/Game/Shadowlightless/BluePrints/Characters/Character_BP` (`|GetArrayItem` (`self.GetOverlappingActors` "/Game/Shadowlightless/BluePrints/Characters/Character_BP.Character_BP_C"))))
          (if (`/Game/Shadowlightless/BluePrints/Characters/Character_BP.bisDead` _ascharacter_bp)
            (set `self.bisattacking` false)
            (else
              (bind _health (`/Game/Shadowlightless/BluePrints/Characters/Character_BP.Health` _ascharacter_bp))
              (if (> _health 0.0)
                (set `/Game/Shadowlightless/BluePrints/Characters/Character_BP.Health` (- _health 5.0) _ascharacter_bp)
                (goto _label_2)
                (else
                  (goto _label_2)))))
          (else
            (set `self.bisattacking` false)
            (goto _label :!via `Reset`)))))))

(event `FollowCharacter`
  (params (Character :type "Character Object Reference"))
  (bind _returnvalue_x (`KismetMathLibrary.BreakVector` (`SceneComponent.K2_GetComponentLocation` (`Character.CapsuleComponent` Character))))
  (bind _returnvalue_x_2 (`KismetMathLibrary.BreakVector` (`SceneComponent.K2_GetComponentLocation` (`self.CapsuleComponent`))))
  (bind _returnvalue (- _returnvalue_x _returnvalue_x_2))
  ;[1 1 1] Follow Character Event
  (if (>= _returnvalue 0.0)
    (set `self.bisMovingRight` true)
    (else
      (set `self.bisMovingRight` false)))
  (`self.AddMovementInput` (1.0 0.0 0.0) _returnvalue))

(event `self.Attack_Collision.OnComponentEndOverlap`
  (params (OverlappedComponent :type "PrimitiveComponent Object Reference") (OtherActor :type "Actor Object Reference") (OtherComp :type "PrimitiveComponent Object Reference") (OtherBodyIndex :type Integer))
  ;[1 1 1] Collisions Overlapping
  (if (`ActorComponent.ComponentHasTag` OtherComp "Hitbox")
    (set `self.isOverlappingAttack` false)))

(event `DeathAnimation`
  (params (DeathAnim :type "PaperFlipbook Object Reference") (DeathAnimLopp :type "PaperFlipbook Object Reference"))
  ;[1 1 1] Death Animation Event
  (`/Engine/EditorBlueprintResources/StandardMacros.DoOnce` false
    (:`Completed`
      (`PaperFlipbookComponent.SetFlipbook` (`self.Sprite`) DeathAnim)
      (`self.DisableInput` null)
      (`KismetSystemLibrary.Delay` 0.667)
      (`PaperFlipbookComponent.SetFlipbook` (`self.Sprite`) DeathAnimLopp)
      (`KismetSystemLibrary.Delay` 0.5))))

(event `RotateEvent`
  ;[1 1 1] Set Enemy Orientation
  (bind _output_get (set `self.X_Velocity` (.x (`MovementComponent.Velocity` (`self.GetMovementComponent`)))))
  (`/Engine/EditorBlueprintResources/StandardMacros.CompareFloat` _output_get
    (:`>`
      (`self.K2_SetActorRotation` (`KismetMathLibrary.MakeRotator` 0.0) :!label _label_3))
    (:`==`
      (if (`self.bisMovingRight`)
        (goto _label_3)
        (else
          (`self.K2_SetActorRotation` (`KismetMathLibrary.MakeRotator` 0.0 0.0 180.0) :!label _label_4))))
    (:`<`
      (goto _label_4))))

(fn `UserConstructionScript`)