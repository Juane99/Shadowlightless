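; Ninja character Blueprint, a child class that supplies Ninja-specific sound and animations to inherited character logic.
; Its attack sound, death, attack and animation-update events call the parent versions, passing in the sword cue and animations for attacks, death, slide, idle, run and jump.
; BeginPlay, Tick and the construction script only forward to the parent, so all behavior logic lives outside this asset.
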(event `self.ReceiveBeginPlay`
  ;[1 1 1] Event Tick & BeginPlay
  (`parent.ReceiveBeginPlay`))

(event `self.ReceiveTick`
  (params (DeltaSeconds :type "Float (single-precision)"))
  ;[1 1 1] Event Tick & BeginPlay
  (`parent.ReceiveTick` DeltaSeconds))

(event `self.PlayAttackSound`
  (params (Sound :type "SoundBase Object Reference"))
  ;[1 1 1] Sounds
  (`parent.PlayAttackSound` "/Game/Shadowlightless/Sounds/sword_Cue.sword_Cue"))

(event `self.DeathAnimationEvent`
  (params (DeathAnim :type "PaperFlipbook Object Reference") (DeathLoopAnim :type "PaperFlipbook Object Reference"))
  ;[1 1 1] Animations
  (`parent.DeathAnimationEvent` "/Game/Shadowlightless/FlipBooks/Characters/Ninja/A_Dead.A_Dead" "/Game/Shadowlightless/FlipBooks/Characters/Ninja/DeadLoop.DeadLoop"))

(event `self.AttackEvent`
  (params (Attack :type "PaperFlipbook Object Reference") (JumpAttack :type "PaperFlipbook Object Reference"))
  ;[1 1 1] Animations
  (`parent.AttackEvent` "/Game/Shadowlightless/FlipBooks/Characters/Ninja/A_Attack.A_Attack" "/Game/Shadowlightless/FlipBooks/Characters/Ninja/A_Jump_Attack.A_Jump_Attack"))

(event `self.UpdateAnimation`
  (params (Slide :type "PaperFlipbook Object Reference") (Idle :type "PaperFlipbook Object Reference") (Run :type "PaperFlipbook Object Reference") (Jump :type "PaperFlipbook Object Reference") (JumpLoop :type "PaperFlipbook Object Reference"))
  ;[1 1 1] Animations
  (`parent.UpdateAnimation` "/Game/Shadowlightless/FlipBooks/Characters/Ninja/A_Slide.A_Slide" "/Game/Shadowlightless/FlipBooks/Characters/Ninja/A_Idle.A_Idle" "/Game/Shadowlightless/FlipBooks/Characters/Ninja/A_Run.A_Run" "/Game/Shadowlightless/FlipBooks/Characters/Ninja/A_Jump.A_Jump" "/Game/Shadowlightless/FlipBooks/Characters/Ninja/A_JumpLoop.A_JumpLoop"))

(fn `UserConstructionScript`
  (`parent.UserConstructionScript`))