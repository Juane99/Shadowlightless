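; Fighter character Blueprint that serves as an animation variant of a parent character class, which handles the underlying logic.
; It overrides the death, attack and animation update events only to pass its animation assets to the parent versions.
; DBZ assets cover idle, flying as the run, attack and death, with shared clips for ground/jump attacks and death/death loop, while slide and jump use A_ assets.
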(event `self.ReceiveBeginPlay`
  ;[1 1 1] Event Tick & BeginPlay
  (`parent.ReceiveBeginPlay`))

(event `self.ReceiveTick`
  (params (DeltaSeconds :type "Float (single-precision)"))
  ;[1 1 1] Event Tick & BeginPlay
  (`parent.ReceiveTick` DeltaSeconds))

(event `self.DeathAnimationEvent`
  (params (DeathAnim :type "PaperFlipbook Object Reference") (DeathLoopAnim :type "PaperFlipbook Object Reference"))
  ;[1 1 1] Animations
  (`parent.DeathAnimationEvent` "/Game/Shadowlightless/FlipBooks/Characters/Fighter/DBZ_Death.DBZ_Death" "/Game/Shadowlightless/FlipBooks/Characters/Fighter/DBZ_Death.DBZ_Death"))

(event `self.AttackEvent`
  (params (Attack :type "PaperFlipbook Object Reference") (JumpAttack :type "PaperFlipbook Object Reference"))
  ;[1 1 1] Animations
  (`parent.AttackEvent` "/Game/Shadowlightless/FlipBooks/Characters/Fighter/DBZ_Attack.DBZ_Attack" "/Game/Shadowlightless/FlipBooks/Characters/Fighter/DBZ_Attack.DBZ_Attack"))

(event `self.UpdateAnimation`
  (params (Slide :type "PaperFlipbook Object Reference") (Idle :type "PaperFlipbook Object Reference") (Run :type "PaperFlipbook Object Reference") (Jump :type "PaperFlipbook Object Reference") (JumpLoop :type "PaperFlipbook Object Reference"))
  ;[1 1 1] Animations
  (`parent.UpdateAnimation` "/Game/Shadowlightless/FlipBooks/Characters/Ninja/A_Slide.A_Slide" "/Game/Shadowlightless/FlipBooks/Characters/Fighter/DBZ_Idle.DBZ_Idle" "/Game/Shadowlightless/FlipBooks/Characters/Fighter/DBZ_Fly.DBZ_Fly" "/Game/Shadowlightless/FlipBooks/Characters/Ninja/A_Jump.A_Jump" "/Game/Shadowlightless/FlipBooks/Characters/Ninja/A_JumpLoop.A_JumpLoop"))

(fn `UserConstructionScript`
  (`parent.UserConstructionScript`))