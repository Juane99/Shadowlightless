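; Indiana_BP is a character Blueprint that supplies Indiana-specific animations, sound and thrown item to a shared parent character class.
; Each event only calls its parent version, passing in Indiana assets for idle, run, jump, melee attack, throw and death animations.
; Initialize sets PossessPlayer_Cue as the attack sound and Kunai as the thrown item, while all gameplay logic stays in the parent.
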(event `self.ReceiveBeginPlay`
  ;[1 1 1] Event Tick & BeginPlay
  (`parent.ReceiveBeginPlay`))

(event `self.ReceiveTick`
  (params (DeltaSeconds :type "Float (single-precision)"))
  ;[1 1 1] Event Tick & BeginPlay
  (`parent.ReceiveTick` DeltaSeconds))

(event `self.Initialize`
  (params (Attack_Sound :type "SoundCue Object Reference") (ThrowedItem :type "Actor Class Reference"))
  ;[1 1 1] Sounds
  (`parent.Initialize` "/Engine/EditorSounds/GamePreview/PossessPlayer_Cue.PossessPlayer_Cue" "/Game/Shadowlightless/BluePrints/Characters/Ninja/Kunai.Kunai_C"))

(event `self.DeathAnimationEvent`
  (params (DeathAnim :type "PaperFlipbook Object Reference") (DeathLoopAnim :type "PaperFlipbook Object Reference") (DeathAnimDuration :type "Float (single-precision)"))
  ;[1 1 1] Animations
  (`parent.DeathAnimationEvent` "/Game/Shadowlightless/FlipBooks/Characters/Indiana/Indi_Dead.Indi_Dead" "/Game/Shadowlightless/FlipBooks/Characters/Indiana/Indi_DeadLoop.Indi_DeadLoop" 0.6))

(event `self.AttackEvent`
  (params (Attack :type "PaperFlipbook Object Reference") (JumpAttack :type "PaperFlipbook Object Reference"))
  ;[1 1 1] Animations
  (`parent.AttackEvent` "/Game/Shadowlightless/FlipBooks/Enemies/Robot/A_Melee.A_Melee" "/Game/Shadowlightless/FlipBooks/Enemies/Robot/A_JumpMelee.A_JumpMelee"))

(event `self.UpdateAnimation`
  (params (Idle :type "PaperFlipbook Object Reference") (Run :type "PaperFlipbook Object Reference") (Jump :type "PaperFlipbook Object Reference") (JumpLoop :type "PaperFlipbook Object Reference"))
  ;[1 1 1] Animations
  (`parent.UpdateAnimation` "/Game/Shadowlightless/FlipBooks/Characters/Indiana/Indi_Idle.Indi_Idle" "/Game/Shadowlightless/FlipBooks/Characters/Indiana/Indi_Run.Indi_Run" "/Game/Shadowlightless/FlipBooks/Characters/Indiana/Indi_Jump.Indi_Jump" "/Game/Shadowlightless/FlipBooks/Characters/Indiana/Indi_JumpLoop.Indi_JumpLoop"))

(event `self.ThrowEvent`
  (params (ThrowAnim :type "PaperFlipbook Object Reference") (JumpThrowAnim :type "PaperFlipbook Object Reference"))
  ;[1 1 1] Animations
  (`parent.ThrowEvent` "/Game/Shadowlightless/FlipBooks/Enemies/Robot/A_Shoot.A_Shoot" "/Game/Shadowlightless/FlipBooks/Enemies/Robot/A_JumpShoot.A_JumpShoot"))

(fn `UserConstructionScript`
  (`parent.UserConstructionScript`))